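; BP_Mech005_Vehicle is a Mech005 vehicle Blueprint that, as written, only runs a frame counter, with no movement or vehicle logic.
; Tick increments an integer and resets it to zero upon reaching 50.
; A helper sets the TextRender component's text, but its only callers, a three-second wait readout, are disconnected, as is an alternative counter based on game time in seconds.
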(event EventTick
  (params (DeltaSeconds :type Float%20%28single-precision%29))
  (Utilities|FlowControl|Sequence
    (:then_1
      ;[1 1 1] counts per 50 frames
      (if (== (Variables|Default|Geti) 50)
        (Variables|Default|Seti 0)
        (else
          (bind _result (Math|Integer|IncrementInt (Variables|Default|Geti))
            (:%20%20
              (Variables|Default|Seti _result))))))))

(fn ConstructionScript)

(fn TextRender
  (params (Text :type Text))
  (Rendering|Components|TextRender|SetText (Variables|Default|GetTextRender) Text))