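; Prototype material-change actor that spins a static mesh and randomizes a shared base color.
; A ResolveMesh timeline started on BeginPlay drives world yaw from its Revolution track, while the construction script sets yaw from ZaxisRotation.
; A Tick frame counter periodically writes random-stream RGB values to the MPC_ChangeBaseColor parameter collection, so the timing depends on frame rate.
; Player 0 input is enabled so the E key triggers the same color change immediately.
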(event EventBeginPlay
  (Utilities|FlowControl|Sequence
    (:then_0
      (Input|EnableInput (Game|GetPlayerController 0)))
    (:then_1
      (bind _revolution (Timeline|Resolve%20Mesh PlayFromStart)
        (:Update
          (Transformation|SetWorldRotation (Variables|Debug|GetStaticMeshComponent) (Math|Rotator|MakeRotator 0.0 0.0 (* _revolution 3.6e+02)) false false))))))

(event EventTick
  (params (DeltaSeconds :type Float%20%28single-precision%29))
  (if (== (Variables|Default|GetCounter) 60)
    (Variables|Default|SetCounter 0)
    (Rendering|Material|SetVectorParameterValue "/Game/Prototyping/Materials/MPC_ChangeBaseColor.MPC_ChangeBaseColor" "BaseColor" (Math|Color|MakeColor (Math|Random|RandomFloatinRangefromStream 0.0 1.0 (Variables|Default|GetRandom_0)) (Math|Random|RandomFloatinRangefromStream 0.0 1.0 (Variables|Default|GetRandom_1)) (Math|Random|RandomFloatinRangefromStream 0.0 1.0 (Variables|Default|GetRandom_2))) :!class /Script/Engine.KismetMaterialLibrary)
    (else
      (bind _result (Math|Integer|IncrementInt (Variables|Default|GetCounter))
        (:%20%20
          (Variables|Default|SetCounter _result))))))

(event Input|KeyboardEvents|E
  (params (Key :type Key%20Structure :default "None"))
  (:Pressed
    (Rendering|Material|SetVectorParameterValue "/Game/Prototyping/Materials/MPC_ChangeBaseColor.MPC_ChangeBaseColor" "BaseColor" (Math|Color|MakeColor (Math|Random|RandomFloatinRangefromStream 0.0 1.0 (Variables|Default|GetRandom_0)) (Math|Random|RandomFloatinRangefromStream 0.0 1.0 (Variables|Default|GetRandom_1)) (Math|Random|RandomFloatinRangefromStream 0.0 1.0 (Variables|Default|GetRandom_2))) :!class /Script/Engine.KismetMaterialLibrary)))

(event Input|KeyboardEvents|R
  (params (Key :type Key%20Structure :default "None")))

(fn ConstructionScript
  (Transformation|SetWorldRotation (Variables|Debug|GetStaticMeshComponent) (Math|Rotator|MakeRotator 0.0 0.0 (Variables|Default|GetZ-axis%20Rotation)) false false))