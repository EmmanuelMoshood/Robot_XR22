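; Prototype character Blueprint that spins its skeletal mesh and relocates it randomly on a key press.
; BeginPlay enables input from the first player controller and starts a timeline whose curve, scaled to degrees, drives the mesh's world yaw.
; Pressing E moves the mesh to a random world XY point within a square around the origin at zero height, using separate random streams per axis.
; The construction script sets initial yaw from ZaxisRotation.
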(event EventBeginPlay
  (Utilities|FlowControl|Sequence
    (:then_0
      (Input|EnableInput (Game|GetPlayerController 0)))
    (:then_1
      (bind _animation_curve_1 (Timeline|Timeline_0 PlayFromStart)
        (:Update
          (Transformation|SetWorldRotation (Variables|SkeletalMeshActor|GetSkeletalMeshComponent) (Math|Rotator|MakeRotator 0.0 0.0 (* _animation_curve_1 3.6e+02)) false false))))))

(event Input|KeyboardEvents|E
  (params (Key :type Key%20Structure :default "None"))
  (:Pressed
    (Transformation|SetWorldLocation (Variables|SkeletalMeshActor|GetSkeletalMeshComponent) (Math|Conversions|ToVector(Float) (Utilities|Struct|MakeIntVector (Math|Random|RandomIntegerinRangefromStream -200 200 (Variables|Default|GetRandom_0)) (Math|Random|RandomIntegerinRangefromStream -200 200 (Variables|Default|GetRandom_1)))) false false)))

(fn ConstructionScript
  (Transformation|SetWorldRotation (Variables|SkeletalMeshActor|GetSkeletalMeshComponent) (Math|Rotator|MakeRotator 0.0 0.0 (Variables|Default|GetZ-axis%20Rotation)) false false))