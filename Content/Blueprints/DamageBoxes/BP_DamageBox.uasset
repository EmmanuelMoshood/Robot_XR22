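; BP_DamageBox is a fire-storm hazard volume that deals periodic damage to the player character standing inside it.
; It spawns a fire storm particle effect at its location on BeginPlay.
; Overlapping DamageBox with a BP_ThirdPersonCharacter stores the character and starts a looping timer that applies damage and prints the result, and end overlap clears that timer.
; A disconnected health-decrement branch is left unused.
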(event OnComponentBeginOverlap(DamageBox)
  (params (OverlappedComponent :type Primitive%20Component%20Object%20Reference) (OtherActor :type Actor%20Object%20Reference) (OtherComp :type Primitive%20Component%20Object%20Reference) (OtherBodyIndex :type Integer) (bFromSweep :type Boolean) (SweepResult :type Hit%20Result%20Structure%20%28by%20ref%29))
  (bind _asbp_third_person_character (Utilities|Casting|CastToBP_ThirdPersonCharacter OtherActor))
  (Variables|Default|SetAs%20BP%20Third%20Person%20Character _asbp_third_person_character)
  (bind _returnvalue (Utilities|Time|SetTimerbyEvent (delegate Custom|DamagePlayer) 1.4 true))
  (Variables|Default|SetTimerRef _returnvalue))

(event OnComponentEndOverlap(DamageBox)
  (params (OverlappedComponent :type Primitive%20Component%20Object%20Reference) (OtherActor :type Actor%20Object%20Reference) (OtherComp :type Primitive%20Component%20Object%20Reference) (OtherBodyIndex :type Integer))
  (Utilities|Casting|CastToBP_ThirdPersonCharacter OtherActor)
  (Utilities|Time|ClearandInvalidateTimerbyHandle (Variables|Default|GetTimerRef)))

(event Custom|DamagePlayer
  (bind _returnvalue (Game|Damage|ApplyDamage (Variables|Default|GetAs%20BP%20Third%20Person%20Character) 25.0 0 0))
  (Development|PrintString (Utilities|String|ToString(Float) _returnvalue) true true "(R=0.000000,G=0.660000,B=1.000000,A=1.000000)" 1.0))

(event EventBeginPlay
  (Effects|SpawnEmitteratLocation "/Game/VFX/FXVarietyPack/Particles/P_ky_fireStorm.P_ky_fireStorm" (Transformation|GetActorLocation)))

(fn ConstructionScript)